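; BP_HappyDoor is a double sliding door prop with open, close and toggle events.
; OpenDoor plays DoorAnimTimeline from the start, while CloseDoor plays a separately named Timeline in reverse from the end.
; Both feed UpdateDoorPosition, which slides the right and left panels in opposite directions along local X.
; ToggleDoor infers the current state from the right panel's X offset instead of storing a flag.
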(event Custom|OpenDoor
  (bind _doorposition (Timeline|DoorAnimTimeline PlayFromStart)
    (:Update
      (CallFunction|UpdateDoorPosition _doorposition))))

(event Custom|ToggleDoor
  (if (< (.X (Math|Vector|BreakVector (Variables|/Script/Engine.SceneComponent|GetRelativeLocation (Variables|Default|GetRightDoor)))) 1.0)
    (CallFunction|OpenDoor)
    (else
      (CallFunction|CloseDoor))))

(event Custom|CloseDoor
  (bind _doorposition (Timeline|Timeline ReverseFromEnd)
    (:Update
      (CallFunction|UpdateDoorPosition _doorposition))))

(event EventBeginPlay)

(event Collision|EventActorBeginOverlap
  (params (OtherActor :type Actor%20Object%20Reference)))

(event EventTick
  (params (DeltaSeconds :type Float%20%28single-precision%29)))

(fn ConstructionScript)

(fn UpdateDoorPosition
  (params (Position :type Float%20%28double-precision%29))
  (bind _rightdoor (Variables|Default|GetRightDoor))
  (bind _leftdoor (Variables|Default|GetLeftDoor))
  (bind _relativelocation (Variables|/Script/Engine.SceneComponent|GetRelativeLocation _rightdoor))
  (bind _relativelocation_2 (Variables|/Script/Engine.SceneComponent|GetRelativeLocation _leftdoor))
  (bind (_x _y _z) (Class|KismetMathLibrary|BreakVector3f _relativelocation_2))
  (bind (_x_2 _y_2 _z_2) (Class|KismetMathLibrary|BreakVector3f _relativelocation))
  (Transformation|SetRelativeLocation _rightdoor (Math|Vector|MakeVector Position _y_2 _z_2) false false)
  (Transformation|SetRelativeLocation _leftdoor (Math|Vector|MakeVector (* Position -1.0) _y _z) false false))