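; Trigger action that gives a target actor a randomized physics impulse when executed.
; It scales ForceVector up or down by a random amount within RandomFactor, keeping the vector's axis.
; The impulse hits the actor's primitive component at its world location, offset by its bounds extent times a random signed scalar, so off-center hits can add spin.
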(event EventExecuteAction
  (params (bInHasOwner :type Boolean) (InOwner :type Actor%20Object%20Reference) (bInHasActivator :type Boolean) (InActivator :type Actor%20Object%20Reference))
  (bind _target_actor (Variables|Default|GetTarget%20Actor))
  (bind _returnvalue (Actor|GetComponentbyClass _target_actor "/Script/Engine.PrimitiveComponent"))
  (Physics|AddImpulseatLocation _returnvalue (+ (Variables|Default|GetForce%20Vector) (* (Variables|Default|GetForce%20Vector) (* (Variables|Default|GetRandom%20Factor) (* (- (Math|Random|RandomFloat) 0.5) 2.0)))) (+ (* (.BoxExtent (Collision|GetComponentBounds _returnvalue)) (* (- (Math|Random|RandomFloat) 0.5) 2.0)) (Transformation|GetWorldLocation _returnvalue)) "None"))